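; BP_Water is a water source, filed under Well, that refills the ThirdPersonCharacter's WaterLevel while overlapped.
; Begin and end overlap on its Collsion component toggle an Overlapping flag for any actor, with begin also caching the cast character.
; While the flag is set, Tick passes a short Delay, re-casts the overlapping actor and adds one to WaterLevel unless it equals exactly 100.
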(event OnComponentBeginOverlap(Collsion)
  (params (OverlappedComponent :type Primitive%20Component%20Object%20Reference) (OtherActor :type Actor%20Object%20Reference) (OtherComp :type Primitive%20Component%20Object%20Reference) (OtherBodyIndex :type Integer) (bFromSweep :type Boolean) (SweepResult :type Hit%20Result%20Structure%20%28by%20ref%29))
  (Variables|Default|SetOverlapping true)
  (bind _asthird_person_character (Utilities|Casting|CastToThirdPersonCharacter OtherActor))
  (bind _output_get (Variables|Default|SetAs%20Third%20Person%20Character _asthird_person_character)))

(event OnComponentEndOverlap(Collsion)
  (params (OverlappedComponent :type Primitive%20Component%20Object%20Reference) (OtherActor :type Actor%20Object%20Reference) (OtherComp :type Primitive%20Component%20Object%20Reference) (OtherBodyIndex :type Integer))
  (Variables|Default|SetOverlapping false))

(event EventTick
  (params (DeltaSeconds :type Float%20%28single-precision%29))
  (if (Variables|Default|GetOverlapping)
    (Utilities|FlowControl|Delay 0.01)
    (Utilities|Casting|CastToThirdPersonCharacter (stale OnComponentBeginOverlap(Collsion) OtherActor))
    (if (not (== (Variables|/Game/ThirdPersonBP/Blueprints/ThirdPersonCharacter.ThirdPersonCharacter_C|GetWaterLevel (Variables|Default|GetAs%20Third%20Person%20Character)) 1e+02))
      (Variables|/Game/ThirdPersonBP/Blueprints/ThirdPersonCharacter.ThirdPersonCharacter_C|SetWaterLevel (stale OnComponentBeginOverlap(Collsion) _output_get) (+ (Variables|/Game/ThirdPersonBP/Blueprints/ThirdPersonCharacter.ThirdPersonCharacter_C|GetWaterLevel (Variables|Default|GetAs%20Third%20Person%20Character)) 1.0)))))

(fn ConstructionScript)