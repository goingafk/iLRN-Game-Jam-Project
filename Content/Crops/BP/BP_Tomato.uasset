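; Tomato crop Blueprint that the player pays to plant, waters halfway through growth, and harvests for money and a tomato count.
; Box overlap caches the ThirdPersonCharacter's money and water, which gate growth along with an Interactions stage counter.
; Delayed Tick runs NewGrowingScript, raising Growth and scaling the cube to match.
; DoOnce nodes limit money and water charges, and harvest resets the crop.
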(event OnComponentBeginOverlap(Box)
  (params (OverlappedComponent :type Primitive%20Component%20Object%20Reference) (OtherActor :type Actor%20Object%20Reference) (OtherComp :type Primitive%20Component%20Object%20Reference) (OtherBodyIndex :type Integer) (bFromSweep :type Boolean) (SweepResult :type Hit%20Result%20Structure%20%28by%20ref%29))
  (bind _output_get (Variables|Default|SetOther%20Actor OtherActor))
  (bind _asthird_person_character (Utilities|Casting|CastToThirdPersonCharacter _output_get))
  (Variables|Default|SetWaterLevels (Variables|/Game/ThirdPersonBP/Blueprints/ThirdPersonCharacter.ThirdPersonCharacter_C|GetWaterLevel _asthird_person_character))
  (Variables|Default|SetMoney (Variables|/Game/ThirdPersonBP/Blueprints/ThirdPersonCharacter.ThirdPersonCharacter_C|GetMoney _asthird_person_character)))

(event OnComponentEndOverlap(Box)
  (params (OverlappedComponent :type Primitive%20Component%20Object%20Reference) (OtherActor :type Actor%20Object%20Reference) (OtherComp :type Primitive%20Component%20Object%20Reference) (OtherBodyIndex :type Integer))
  (Variables|Default|SetOther%20Actor (Variables|Default|GetEmpty)))

(event Custom|NewGrowingScript
  (bind _cube (Variables|Default|GetCube))
  (bind _cube_2 (Variables|Default|GetCube))
  (if (and (> (Variables|Default|GetInteractions) 0) (or (>= (Variables|Default|GetMoney) 2) (Variables|Default|GetPaid)))
    (Variables|Default|SetPaid true)
    (Utilities|FlowControl|Sequence
      (:then_0
        (Utilities|FlowControl|DoOnce false :!label _label
          (:Completed
            (bind _asthird_person_character (Utilities|Casting|CastToThirdPersonCharacter (Variables|Default|GetOther%20Actor)))
            (Variables|/Game/ThirdPersonBP/Blueprints/ThirdPersonCharacter.ThirdPersonCharacter_C|SetMoney _asthird_person_character (- (Variables|/Game/ThirdPersonBP/Blueprints/ThirdPersonCharacter.ThirdPersonCharacter_C|GetMoney _asthird_person_character) 2)))))
      (:then_1
        (Rendering|SetVisibility (Variables|Default|GetCube) true false)
        (if (>= (Variables|Default|GetGrowth) 0.5)
          (if (and (> (Variables|Default|GetInteractions) 1) (>= (Variables|Default|GetGrowth) 0.5))
            (if (not (>= (Variables|Default|GetGrowth) 1.0))
              (if (>= (Variables|Default|GetWaterLevels) 3e+01)
                (Variables|Default|SetGrowth (+ (Variables|Default|GetGrowth) 0.01))
                (Variables|Default|SetInteractions 2)
                (Variables|Default|SetisWatered true)
                (Utilities|FlowControl|DoOnce false :!label _label_2
                  (:Completed
                    (bind _asthird_person_character_2 (Utilities|Casting|CastToThirdPersonCharacter (Variables|Default|GetOther%20Actor)))
                    (Variables|/Game/ThirdPersonBP/Blueprints/ThirdPersonCharacter.ThirdPersonCharacter_C|SetWaterLevel _asthird_person_character_2 (- (Variables|Default|GetWaterLevels) 3e+01))))
                (else
                  (Rendering|SetVisibility (Variables|Default|GetNeedWater) true false)
                  (if (<= (Variables|Default|GetWaterLevels) 3e+01)
                    (Variables|Default|SetInteractions 2))))
              (elif (>= (Variables|Default|GetInteractions) 3)
                (bind _output_get (Variables|Default|SetGrowth 0.1))
                (Transformation|SetRelativeScale3D _cube (Math|Conversions|ToVector(Float) _output_get))
                (Rendering|SetVisibility _cube false false)
                (Variables|Default|SetInteractions 0)
                (Variables|Default|SetPaid false)
                (Rendering|SetVisibility (Variables|Default|GetNeedWater) false false)
                (bind _asthird_person_character_3 (Utilities|Casting|CastToThirdPersonCharacter (Variables|Default|GetOther%20Actor)))
                (Variables|/Game/ThirdPersonBP/Blueprints/ThirdPersonCharacter.ThirdPersonCharacter_C|SetMoney _asthird_person_character_3 (+ 4 (Variables|/Game/ThirdPersonBP/Blueprints/ThirdPersonCharacter.ThirdPersonCharacter_C|GetMoney _asthird_person_character_3)))
                (Variables|/Game/ThirdPersonBP/Blueprints/ThirdPersonCharacter.ThirdPersonCharacter_C|SetTomatoCounter _asthird_person_character_3 (+ (Variables|/Game/ThirdPersonBP/Blueprints/ThirdPersonCharacter.ThirdPersonCharacter_C|GetTomatoCounter _asthird_person_character_3) 1))
                (Utilities|FlowControl|Sequence
                  (:then_0
                    (goto _label Reset))))))
          (else
            (Variables|Default|SetGrowth (+ (Variables|Default|GetGrowth) 0.01))
            (Variables|Default|SetInteractions 1)))))
    (else
      (Transformation|SetRelativeScale3D _cube_2 "0.100000,0.100000,0.100000")
      (Rendering|SetVisibility _cube_2 false false)
      (goto _label_2 Reset))))

(event EventTick
  (params (DeltaSeconds :type Float%20%28single-precision%29))
  (Utilities|FlowControl|Delay 0.1)
  (CallFunction|NewGrowingScript)
  (Transformation|SetRelativeScale3D (Variables|Default|GetCube) (Math|Conversions|ToVector(Float) (Variables|Default|GetGrowth))))

(fn ConstructionScript)